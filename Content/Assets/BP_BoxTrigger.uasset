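; Trigger volume that shows a meeting-selection menu (WBP_SelectMeeting) while the local first-person character stands inside it.
; On begin overlap it creates the widget, passes it the first BP_SitTargetPrivate and BP_SitTargetAI found in the level as private and AI interview targets, and adds it to the viewport.
; On end overlap it removes the stored widget.
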(event `self.ReceiveActorBeginOverlap`
  (params (OtherActor :type "Actor Object Reference"))
  (bind _selectmeetingwidgetref (`self.SelectMeetingWidgetRef`))
  (bind _asbp_first_person_character (cast `/Game/FirstPerson/Blueprints/BP_FirstPersonCharacter` OtherActor)
    (:`then`
      (if (`Controller.IsLocalController` (`Pawn.GetController` _asbp_first_person_character))
        (bind _returnvalue (`|CreateWidget` "/Game/UI/WBP_SelectMeeting.WBP_SelectMeeting_C" (`GameplayStatics.GetPlayerController` 0)))
        (set `self.SelectMeetingWidgetRef` _returnvalue)
        (bind _returnvalue_2 (`GameplayStatics.GetActorOfClass` "/Game/Assets/BP_SitTargetPrivate.BP_SitTargetPrivate_C"))
        (bind _returnvalue_3 (`GameplayStatics.GetActorOfClass` "/Game/Assets/BP_SitTargetAI.BP_SitTargetAI_C"))
        (`Rene_SelectMeetingWidget.SetTargetActors` _selectmeetingwidgetref _returnvalue_2 _returnvalue_3)
        (`UserWidget.AddToViewport` _selectmeetingwidgetref 0)))
    (:`CastFailed`
      (`KismetSystemLibrary.PrintString` "fail" :!label _label))))

(event `self.ReceiveActorEndOverlap`
  (params (OtherActor :type "Actor Object Reference"))
  (bind _selectmeetingwidgetref (`self.SelectMeetingWidgetRef`))
  (bind _asbp_first_person_character (cast `/Game/FirstPerson/Blueprints/BP_FirstPersonCharacter` OtherActor)
    (:`then`
      (if (`Controller.IsLocalController` (`Pawn.GetController` _asbp_first_person_character))
        (`/Engine/EditorBlueprintResources/StandardMacros.IsValid` _selectmeetingwidgetref
          (:`Is Valid`
            (`Widget.RemoveFromParent` _selectmeetingwidgetref)))))
    (:`CastFailed`
      (goto _label))))

(fn `UserConstructionScript`)