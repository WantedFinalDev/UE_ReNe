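; Player controller Blueprint that sets up the front-end UI and camera when it possesses a pawn.
; On possess it creates the primary layout widget, registers it with the FE UI subsystem, and pushes the tag-resolved Login soft widget onto the FrontEnd stack on every map.
; SetCam switches the view to a "Default"-tagged CameraActor on StartMap.
; Its branch for other maps, noted for a HUD push, is empty.
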(event `self.ReceivePossess`
  (params (PossessedPawn :type "Pawn Object Reference"))
  (`self.SetCam`)
  (bind _returnvalue (`|CreateWidget` "/Game/Blueprints/FE/Widgets/WBP_CUW_PrimaryLayout.WBP_CUW_PrimaryLayout_C" self))
  (`UserWidget.AddToViewport` _returnvalue 0)
  (`FE_UISubsystem.RegisterCreatedPrimaryLayout` (subsystem `FE_UISubsystem`) _returnvalue)
  (`AsyncAction_PushSoftWidget.PushSoftWidget` self (`FE_FunctionLibrary.GetFESoftWidgetClassByTag` (struct :`TagName` "FE.Widget.Login")) (struct :`TagName` "FE.WidgetStack.FrontEnd")))

(fn `SetCam`
  (bind _returnvalue (`GameplayStatics.GetCurrentLevelName` true))
  (if (`KismetStringLibrary.EqualEqual_StrStr` _returnvalue "StartMap")
    (bind _outactors (`GameplayStatics.GetAllActorsOfClassWithTag` "/Script/Engine.CameraActor" "Default"))
    (if (not (`KismetArrayLibrary.Array_IsEmpty` _outactors))
      (`self.SetViewTargetWithBlend` (`|GetArrayItem` _outactors)))
    (else
      ; false  : HUD Push
      (`|ExecutionSequence`))))

(fn `UserConstructionScript`)