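; Parent Blueprint for pressable interactive buttons with a status light and a hover prompt.
; The construction script creates and stores a dynamic material instance on the button mesh's light slot.
; UpdateButtonVisuals sets that material's State scalar to switch the light between green when enabled and red when disabled.
; OnPlayerHover returns a "Press Button" prompt only when the hit component is the button's collision.
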(fn `OnPlayerHover`
  (params (HitResult :type "HitResult Structure"))
  (returns (InteractText :type Text))
  (if (== (`self.ButtonCollision`) (`.HitComponent` (`GameplayStatics.BreakHitResult` HitResult)))
    (return "Press Button")
    (else
      (return ""))))

(fn `UpdateButtonVisuals`
  (params (Enable :type Boolean))
  (bind _button_light_material (`self.Button light material`))
  (if Enable
    (`MaterialInstanceDynamic.SetScalarParameterValue` _button_light_material "State" 1.0) ; Change a scalar value in the button material that turns it green
    (else
      (`MaterialInstanceDynamic.SetScalarParameterValue` _button_light_material "State" 0.0) ; Change a scalar value in the button material that turns it back to red
    )))

(fn `UserConstructionScript`
  (bind _returnvalue (`PrimitiveComponent.CreateDynamicMaterialInstance` (`self.ButtonMesh`) 1 null "None"))
  (set `self.Button light material` _returnvalue) ; Save a reference to the Dynamic Material Instance for use in the event graph
)